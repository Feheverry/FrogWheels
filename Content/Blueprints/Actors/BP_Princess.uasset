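; BP_Princess is the princess actor whose capsule overlap with the Paper2D_Frog player ends the game.
; On overlap it calls the frog's WormKill with a fixed value, destroys its own capsule, switches to the dead princess flipbook and disables the frog's input.
; After a short delay it pauses the game, shows the UI_Finish widget and enables the mouse cursor.
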(event `self.Capsule.OnComponentBeginOverlap`
  (params (OverlappedComponent :type "PrimitiveComponent Object Reference") (OtherActor :type "Actor Object Reference") (OtherComp :type "PrimitiveComponent Object Reference") (OtherBodyIndex :type Integer) (bFromSweep :type Boolean) (SweepResult :type "HitResult Structure (by ref)"))
  (bind _aspaper_2d_frog (cast `/Game/Blueprints/Paper2D_Frog` OtherActor))
  (`/Game/Blueprints/Paper2D_Frog.WormKill` _aspaper_2d_frog 100)
  (`ActorComponent.K2_DestroyComponent` (`self.Capsule`))
  (`PaperFlipbookComponent.SetFlipbook` (`self.FB_Princess`) "/Game/Flipbooks/FB_PricessDead.FB_PricessDead")
  (`self.DisableInput` OtherActor null)
  (`KismetSystemLibrary.Delay` 1.0)
  (`GameplayStatics.SetGamePaused` true)
  (bind _returnvalue (`|CreateWidget` "/Game/Blueprints/UI/UI_Finish.UI_Finish_C" (`GameplayStatics.GetPlayerController` 0)))
  (`UserWidget.AddToViewport` _returnvalue 0)
  (set `PlayerController.bShowMouseCursor` true (`GameplayStatics.GetPlayerController` 0)))

(fn `UserConstructionScript`)