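; Paper2D frog player character that moves on the X/Z plane with four-direction idle and run flipbooks.
; Tick calls SetMyFlipbook, which stores the last movement direction from axis input and uses velocity to choose run or idle.
; HealthSystem subtracts damage, briefly locking input, or on death shrinks the sprite and reloads the current level.
; SideTrail and UpDownTrail rotate ArmVFX by movement axis, but nothing here calls them.
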(event `HealthSystem`
  (params (DamageAmount :type "Float (double-precision)" :default 0.2))
  (bind _output_get (set `self.Current Health` (- (`self.Current Health`) DamageAmount)))
  (if (< _output_get 0.1)
    (`self.DisableInput` null)
    (`SceneComponent.SetWorldScale3D` (`self.Sprite`) (0.6 0.6 0.6))
    (`KismetSystemLibrary.Delay` 0.1)
    (`MovementComponent.StopMovementImmediately` (`self.CharacterMovement`))
    (`SceneComponent.SetWorldScale3D` (`self.Sprite`) (0.6 0.6 0.6))
    (`SceneComponent.SetWorldScale3D` (`self.Sprite`) (0.4 0.4 0.4))
    (`SceneComponent.SetWorldScale3D` (`self.Sprite`) (0.3 0.3 0.3))
    (`KismetSystemLibrary.Delay` 0.5)
    (bind _returnvalue (`GameplayStatics.GetCurrentLevelName` true))
    (`GameplayStatics.OpenLevel` (`KismetStringLibrary.Conv_StringToName` _returnvalue))
    (else
      (`self.DisableInput` (`GameplayStatics.GetPlayerController` 0))
      (`KismetSystemLibrary.Delay` 0.5)
      (`self.EnableInput` null)
      (`self.SetMyFlipbook`))))

(event `self.ReceiveTick`
  (params (DeltaSeconds :type "Float (single-precision)"))
  (`self.SetMyFlipbook`))

(event `InputAxis|UpDownMovement`
  (params (AxisValue :type "Float (single-precision)"))
  (`self.AddMovementInput` (0.0 0.0 1.0) AxisValue))

(event `SideTrail`
  (if (!= (`self.GetInputAxisValue`) 0.0)
    (`SceneComponent.K2_SetWorldRotation` (`self.Arm_VFX`) (struct :`Yaw` 90.0 :`Roll` 90.0) false false)))

(event `InputAxis|RightLeftMovement`
  (params (AxisValue :type "Float (single-precision)"))
  (`self.AddMovementInput` (1.0 0.0 0.0) AxisValue))

(event `UpDownTrail`
  (if (!= (`self.GetInputAxisValue`) 0.0)
    (`SceneComponent.K2_SetWorldRotation` (`self.Arm_VFX`) (struct :`Yaw` 90.0) false false)))

(fn `SetMyFlipbook`
  (bind _lasmoveddir (`self.LasMovedDir`))
  (if (or (!= (`self.GetInputAxisValue`) 0.0) (!= (`self.GetInputAxisValue`) 0.0))
    (set `self.LasMovedDir` (select `bool` (> (`self.GetInputAxisValue`) 0.0) :`false` (select `bool` (< (`self.GetInputAxisValue`) 0.0) :`false` (select `bool` (> (`self.GetInputAxisValue`) 0.0) :`false` "NewEnumerator2" :`true` "NewEnumerator3" :!type "/Game/Blueprints/MoveDir Enum") :`true` "NewEnumerator1") :`true` "NewEnumerator0")))
  (`PaperFlipbookComponent.SetFlipbook` (`self.Sprite`) (select `bool` (> (`KismetMathLibrary.VSize` (`self.GetVelocity`)) 0.0) :`false` (select `/Game/Blueprints/MoveDir` _lasmoveddir :`NewEnumerator0` "/Game/Flipbooks/Idle_U.Idle_U" :`NewEnumerator1` "/Game/Flipbooks/Idle_D.Idle_D" :`NewEnumerator2` "/Game/Flipbooks/Idle_L.Idle_L" :`NewEnumerator3` "/Game/Flipbooks/Idle_R.Idle_R" :!type "PaperFlipbook Object Reference") :`true` (select `/Game/Blueprints/MoveDir` _lasmoveddir :`NewEnumerator0` "/Game/Flipbooks/Run_U.Run_U" :`NewEnumerator1` "/Game/Flipbooks/Run_D.Run_D" :`NewEnumerator2` "/Game/Flipbooks/Run_L.Run_L" :`NewEnumerator3` "/Game/Flipbooks/Run_R.Run_R" :!type "PaperFlipbook Object Reference"))))

(fn `UserConstructionScript`)